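; Lobby game mode that registers joining players, shows them the lobby screen and moves the session to the chosen map.
; On login, the authority stores each controller and passes server name, map and mode from MyGameInstance to LobbyPlayerController's lobby widget call.
; JoinGame issues a servertravel console command for Map1 or Map2, defaulting to Map1, then calls JoinGame on the game instance.
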(event `self.K2_PostLogin`
  (params (NewPlayer :type "PlayerController Object Reference"))
  (`/Engine/EditorBlueprintResources/ActorMacros.Switch Has Authority`
    (:`Authority`
      (`KismetArrayLibrary.Array_Add` (`self.AllPCs`) NewPlayer)
      (bind _asmy_game_instance (cast `/Game/Blueprints/MyGameInstance` (`GameplayStatics.GetGameInstance`)))
      (set `self.ServerName` (`/Game/Blueprints/MyGameInstance.ServerName` _asmy_game_instance))
      (set `self.ServerMap` (`/Game/Blueprints/MyGameInstance.ServerMap` _asmy_game_instance))
      (set `self.ServerMode` (`/Game/Blueprints/MyGameInstance.ServerMode` _asmy_game_instance))
      (bind _aslobby_player_controller (cast `/Game/Blueprints/LobbyPlayerController` NewPlayer))
      (`/Game/Blueprints/LobbyPlayerController.AddLobbyWB` _aslobby_player_controller (`self.ServerName`) (`self.ServerMap`) (`self.ServerMode`)))))

(event `JoinGame`
  (bind _returnvalue (`GameplayStatics.GetPlayerController` 0))
  (if (`KismetStringLibrary.EqualEqual_StrStr` (`self.ServerMap`) "Map1")
    (`KismetSystemLibrary.ExecuteConsoleCommand` "servertravel/Game/Maps/Map1" _returnvalue :!label _label)
    (elif (`KismetStringLibrary.EqualEqual_StrStr` (`self.ServerMap`) "Map2")
      (`KismetSystemLibrary.ExecuteConsoleCommand` "servertravel/Game/Maps/Map2" _returnvalue)
      (else
        (goto _label))))
  (bind _asmy_game_instance (cast `/Game/Blueprints/MyGameInstance` (`GameplayStatics.GetGameInstance`)))
  (`/Game/Blueprints/MyGameInstance.JoinGame` _asmy_game_instance))

(fn `UserConstructionScript`)