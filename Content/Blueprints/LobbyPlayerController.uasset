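; LobbyPlayerController is the player controller for a multiplayer lobby, handling the lobby UI and the switch to a loading screen.
; AddLobbyWB creates the LobbyWB widget with the server name, map and mode converted to text, stores it and adds it to the viewport.
; LoadingScreen removes the stored lobby widget and shows a new LoadingScreen widget owned by this controller.
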(event `AddLobbyWB`
  (params (ServerName :type String) (ServerMap :type String) (ServerMode :type String))
  (bind _returnvalue (`|CreateWidget` "/Game/UI/LobbyWB.LobbyWB_C" null (`KismetTextLibrary.Conv_StringToText` ServerName) (`KismetTextLibrary.Conv_StringToText` ServerMap) (`KismetTextLibrary.Conv_StringToText` ServerMode)))
  (bind _output_get (set `self.LobbyWB` _returnvalue))
  (`UserWidget.AddToViewport` _output_get 1))

(event `LoadingScreen`
  (`Widget.RemoveFromParent` (`self.LobbyWB`))
  (bind _returnvalue (`|CreateWidget` "/Game/UI/LoadingScreen.LoadingScreen_C" self))
  (`UserWidget.AddToViewport` _returnvalue 0))

(fn `UserConstructionScript`)